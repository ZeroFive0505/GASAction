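; Gameplay ability that fires a single hitscan shot from the equipped weapon.
; It plays the weapon's montage and waits once for the Event.Combat.Shoot gameplay event, ending if the montage finishes first.
; The shot line-traces from the muzzle using control rotation, with debug drawing, and plays weapon effects.
; A hit actor with an ability system component receives the weapon's effect spec, then the ability ends.
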(event `self.K2_ActivateAbilityFromEvent`
  (params (EventData :type "GameplayEventData Structure (by ref)"))
  (`AbilityTask_PlayMontageAndWait.CreatePlayMontageAndWaitProxy` "None" (`WeaponStaticData.AnimMontage` (`self.GetEquippedItemWeaponStaticData`))
    (:`then`
      (`AbilityTask_WaitGameplayEvent.WaitGameplayEvent` (struct :`TagName` "Event.Combat.Shoot") null true
        (:`EventReceived`
          (`self.Shoot`))))
    (:`OnCompleted`
      (`self.K2_EndAbility` :!label _label))
    (:`OnBlendOut`
      (goto _label))
    (:`OnInterrupted`
      (goto _label))
    (:`OnCancelled`
      (goto _label))))

(event `Shoot`
  (bind _returnvalue (`WeaponItemActor.GetMuzzlePosition` (`self.GetEquippedWeaponItemActor`)))
  (bind (_outhit _returnvalue_2) (`KismetSystemLibrary.LineTraceSingle` :`Start` _returnvalue :`End` (+ _returnvalue (* (`Controller.GetControlRotation` (`.PlayerController` (break `GameplayAbilityActorInfo` (`self.GetActorInfo`)))) (`self.ShootingDistance`))) :`TraceChannel` "TraceTypeQuery3" :`DrawDebugType` "ForDuration"))
  (`WeaponItemActor.PlayWeaponEffects` (`self.GetEquippedWeaponItemActor`) _outhit)
  (if _returnvalue_2
    (bind _returnvalue_3 (`AbilitySystemBlueprintLibrary.GetAbilitySystemComponent` (`.HitActor` (`GameplayStatics.BreakHitResult` _outhit))))
    (`/Engine/EditorBlueprintResources/StandardMacros.IsValid` _returnvalue_3
      (:`Is Valid`
        (`AbilitySystemComponent.BP_ApplyGameplayEffectSpecToSelf` _returnvalue_3 (`self.GetWeaponEffectSpec` _outhit)))
      (:`Is Not Valid`
        _)))
  (`self.K2_EndAbility`))