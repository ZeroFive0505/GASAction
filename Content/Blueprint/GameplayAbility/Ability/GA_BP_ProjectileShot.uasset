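; Gameplay ability that fires a rocket projectile from the character's equipped weapon.
; On activation, a weapon-to-focus trace supplies the shot direction and feeds a red debug line and the weapon effects.
; The rocket spawns at the muzzle, offset along that direction, with the character as owner and instigator.
; The ability then ends; a failed trace does nothing and never reaches EndAbility.
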(event `self.K2_ActivateAbility`
  (bind _returnvalue (`self.GetActionGameCharacterFromActorInfo`))
  (bind (_outhitresult _returnvalue_2) (`self.GetWeaponToFocusTraceResult` (`self.ShootingDistance`) "TraceTypeQuery3"))
  (bind (_bblockinghit _binitialoverlap _time _distance _location _impactpoint _normal _impactnormal _physmat _hitactor _hitcomponent _hitbonename _bonename _hititem _elementindex _faceindex _tracestart _traceend) (`GameplayStatics.BreakHitResult` _outhitresult))
  (bind _returnvalue_3 (`KismetMathLibrary.Normal` (- _traceend _tracestart)))
  (if _returnvalue_2
    (`KismetSystemLibrary.DrawDebugLine` _tracestart (* _traceend (`self.ShootingDistance`)) (struct :`R` 1.0 :`A` 1.0) 2.0 0.5)
    (`WeaponItemActor.PlayWeaponEffects` (`self.GetEquippedWeaponItemActor`) _outhitresult)
    (`ActionGameStatics.LaunchProjectile` "/Game/Blueprint/Projectile/BP_ProjectileRocketData.BP_ProjectileRocketData_C" (`KismetMathLibrary.MakeTransform` (+ (`WeaponItemActor.GetMuzzlePosition` (`self.GetEquippedWeaponItemActor`)) (* _returnvalue_3 (`self.SpawnOffset`))) (`KismetMathLibrary.Conv_VectorToRotator` _returnvalue_3)) _returnvalue _returnvalue)
    (`self.K2_EndAbility`)))