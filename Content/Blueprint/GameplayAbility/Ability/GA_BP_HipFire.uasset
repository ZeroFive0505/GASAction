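; Gameplay ability for automatic hip fire with the equipped weapon.
; It plays the weapon's montage and loops a fire-rate timer until the attack-ended event arrives or the montage stops, clearing the timer on end.
; Each shot does a debug-drawn Visibility line trace from the muzzle using the controller's control rotation, applying the weapon's damage effect to hit actors with an Ability System Component.
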(event `self.K2_ActivateAbilityFromEvent`
  (params (EventData :type "GameplayEventData Structure (by ref)"))
  (bind _returnvalue (`self.GetEquippedItemWeaponStaticData`))
  (`AbilityTask_PlayMontageAndWait.CreatePlayMontageAndWaitProxy` "None" (`WeaponStaticData.AnimMontage` _returnvalue)
    (:`then`
      (bind _returnvalue_2 (`KismetSystemLibrary.K2_SetTimerDelegate` (delegate `Shoot`) (/ 1.0 (`WeaponStaticData.FireRate` _returnvalue)) true))
      (set `self.ShootTimer` _returnvalue_2)
      (`AbilityTask_WaitGameplayEvent.WaitGameplayEvent` (struct :`TagName` "Event.Combat.Attack.Ended") null
        (:`EventReceived`
          (`self.K2_EndAbility`))))
    (:`OnCompleted`
      (`self.K2_EndAbility` :!label _label))
    (:`OnInterrupted`
      (goto _label))
    (:`OnCancelled`
      (goto _label))))

(event `Shoot`
  (bind _returnvalue (`WeaponItemActor.GetMuzzlePosition` (`self.GetEquippedWeaponItemActor`)))
  (bind (_outhit _returnvalue_2) (`KismetSystemLibrary.LineTraceSingle` :`Start` _returnvalue :`End` (+ _returnvalue (* (`Controller.GetControlRotation` (`.PlayerController` (break `GameplayAbilityActorInfo` (`self.GetActorInfo`)))) (`self.ShootingDistance`))) :`TraceChannel` "TraceTypeQuery1" :`DrawDebugType` "ForDuration"))
  (if _returnvalue_2
    (bind _returnvalue_3 (`AbilitySystemBlueprintLibrary.GetAbilitySystemComponent` (`.HitActor` (`GameplayStatics.BreakHitResult` _outhit))))
    (`/Engine/EditorBlueprintResources/StandardMacros.IsValid` _returnvalue_3
      (:`Is Valid`
        (`AbilitySystemComponent.BP_ApplyGameplayEffectToSelf` :`self` _returnvalue_3 :`GameplayEffectClass` (`WeaponStaticData.DamageEffect` (`self.GetEquippedItemWeaponStaticData`)))))))

(event `self.K2_OnEndAbility`
  (params (bWasCancelled :type Boolean))
  (`KismetSystemLibrary.K2_ClearAndInvalidateTimerHandle` (`self.ShootTimer`)))